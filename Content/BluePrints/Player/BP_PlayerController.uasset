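; Player controller that manages the HUD, the Tab menu and quitting the game with Escape.
; On begin play it shows the HUD's main widget and binds to the tab widget's mesh dispatcher.
; Tab swaps main and tab widgets, switching input mode, cursor and pawn input to match.
; A handler function forwards a mesh to the controlled BP_Player as its current imported mesh.
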(event EventBeginPlay
  ;[0 0 0] Initialize
  (bind _asbp_hud (Utilities|Casting|CastToBP_HUD (HUD|GetHUD)))
  (bind _output_get (Variables|Default|SetHUD_ref _asbp_hud))
  (Default|TogleMainWidget _output_get true)
  (bind _tab_widget_ref (Variables|/Game/BluePrints/UserInterface/HUD/BP_HUD.BP_HUD_C|Gettab_widget_ref _output_get)
    (:then
      (EventDispatchers|BindEventtoMeshBindingDisp _tab_widget_ref (EventDispatchers|CreateEvent :!event BPPlayerControllerAutoGenFunc)))
    (:else)))

(event Input|KeyboardEvents|Tab
  (params (Key :type Key%20Structure :default "None"))
  (bind _returnvalue (Pawn|GetControlledPawn))
  (bind _self self)
  (bind _hud_ref (Variables|Default|GetHUD_ref))
  (bind _hud_ref_2 (Variables|Default|GetHUD_ref))
  ;[0 0 0 0.719] Tab Menu
  (:Pressed
    (if (not (Variables|Default|Getis_tab_menu_active))
      (Variables|Default|Setis_tab_menu_active true)
      (bind _tab_widget_ref (Default|TogleTabWidget _hud_ref true))
      (Input|SetInputModeGameandUI _self _tab_widget_ref "DoNotLock" true)
      (Input|DisableInput _returnvalue 0)
      (Variables|Default|SetbShowMouseCursor true)
      (Default|TogleMainWidget _hud_ref_2 false)
      (else
        (Variables|Default|Setis_tab_menu_active false)
        (Default|TogleTabWidget _hud_ref false)
        (Input|SetInputModeGameOnly _self)
        (Input|EnableInput _returnvalue 0)
        (Variables|Default|SetbShowMouseCursor false)
        (Default|TogleMainWidget _hud_ref_2 true)))))

(event Input|KeyboardEvents|Escape
  (params (Key :type Key%20Structure :default "None"))
  ;[0 0 0] quit
  (:Pressed
    (Game|QuitGame 0 "Quit" false)))

(fn ConstructionScript)

(fn BPPlayerControllerAutoGenFunc
  (params (NewParam :type Text))
  (bind _asbp_player (Utilities|Casting|CastToBP_Player (Pawn|GetControlledPawn)))
  (Default|SetCurrentImportedMesh _asbp_player NewParam))